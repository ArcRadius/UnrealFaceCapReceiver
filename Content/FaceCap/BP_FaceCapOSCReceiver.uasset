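; Actor that receives face capture data over OSC and stores head position, head rotation, both eye rotations and 51 morph target weights.
; When AutoActivate is set it binds to its OscReceiver on BeginPlay; open and close events bind or unbind, guarded by a DoOnce.
; Incoming messages route by address to update functions that check argument count, remap axes and offsets into Unreal space, and print each value for debugging.
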(event Custom|OnOscRx
  (params (Address :type Name%20%28by%20ref%29) (Data :type Array%20of%20Osc%20Data%20Elem%20Struct%20Structures) (SenderIp :type String))
  (switch name Address
    (:/HT
      (CallFunction|UpdateHeadPosition Data))
    (:/HR
      (CallFunction|UpdateHeadRotation Data))
    (:/ELR
      (CallFunction|UpdateLeftEyeRotation Data))
    (:/ERR
      (CallFunction|UpdateRightEyeRotation Data))
    (:/W
      (CallFunction|UpdateBlendShape Data))))

(event Custom|OnCloseOsc
  (bind _oscreceiver (Variables|Default|GetOscReceiver))
  (EventDispatchers|UnbindEventfromOnOscReceived _oscreceiver (delegate Custom|OnOscRx))
  (Utilities|FlowControl|DoOnce false) ; enters at Reset
)

(event Custom|OnOpenOsc
  (Utilities|FlowControl|DoOnce false
    (:Completed
      (EventDispatchers|BindEventtoOnOscReceived (Variables|Default|GetOscReceiver) (delegate Custom|OnOscRx)))))

(event EventBeginPlay
  (if (Variables|Default|GetbAutoActivate)
    (CallFunction|OnOpenOsc)))

(event Collision|EventActorBeginOverlap
  (params (OtherActor :type Actor%20Object%20Reference)))

(event EventTick
  (params (DeltaSeconds :type Float%20%28single-precision%29)))

(fn ConstructionScript
  (Utilities|Array|Resize (Variables|Default|GetMorphValues) 51))

(fn UpdateHeadRotation
  (params (Array :type Array%20of%20Osc%20Data%20Elem%20Struct%20Structures))
  (if (== (Utilities|Array|Length Array) 3)
    (Variables|Default|SetHeadRotation (Math|Rotator|MakeRotator (+ (Class|OscFunctionLibrary|AsFloat (Utilities|Array|Get(acopy) Array)) 9e+01) (Class|OscFunctionLibrary|AsFloat (Utilities|Array|Get(acopy) Array 2)) (Class|OscFunctionLibrary|AsFloat (Utilities|Array|Get(acopy) Array 1))))
    (Development|PrintString (Utilities|String|Append "EulerAngles: " (Utilities|String|ToString(Rotator) (Variables|Default|GetHeadRotation))) false)
    (return)
    (else
      (Development|PrintString "Warning: Received partial blob")
      (return))))

(fn UpdateHeadPosition
  (params (Array :type Array%20of%20Osc%20Data%20Elem%20Struct%20Structures))
  (if (== (Utilities|Array|Length Array) 3)
    (Variables|Default|SetHeadPosition (Math|Vector|MakeVector (* (Class|OscFunctionLibrary|AsFloat (Utilities|Array|Get(acopy) Array)) -1.0) (Class|OscFunctionLibrary|AsFloat (Utilities|Array|Get(acopy) Array 2)) (Class|OscFunctionLibrary|AsFloat (Utilities|Array|Get(acopy) Array 1))))
    (Development|PrintString (Utilities|String|Append "Position: " (Utilities|String|ToString(Vector) (Variables|Default|GetHeadPosition))) false)
    (return)
    (else
      (Development|PrintString "Warning: Received partial blob")
      (return))))

(fn UpdateLeftEyeRotation
  (params (Array :type Array%20of%20Osc%20Data%20Elem%20Struct%20Structures))
  (if (== (Utilities|Array|Length Array) 2)
    (Variables|Default|SetEyeLeft (Math|Rotator|MakeRotator (+ (Class|OscFunctionLibrary|AsFloat (Utilities|Array|Get(acopy) Array)) 9e+01) 0.0 (Class|OscFunctionLibrary|AsFloat (Utilities|Array|Get(acopy) Array 1))))
    (Development|PrintString (Utilities|String|Append "LeftEyeEulerAngles: " (Utilities|String|ToString(Rotator) (Variables|Default|GetEyeLeft))) false)
    (return)
    (else
      (Development|PrintString "Warning: Received partial blob")
      (return))))

(fn UpdateRightEyeRotation
  (params (Array :type Array%20of%20Osc%20Data%20Elem%20Struct%20Structures))
  (if (== (Utilities|Array|Length Array) 2)
    (Variables|Default|SetEyeRight (Math|Rotator|MakeRotator (+ (Class|OscFunctionLibrary|AsFloat (Utilities|Array|Get(acopy) Array)) 9e+01) 0.0 (Class|OscFunctionLibrary|AsFloat (Utilities|Array|Get(acopy) Array 1))))
    (Development|PrintString (Utilities|String|Append "RightEyeEulerAngles: " (Utilities|String|ToString(Rotator) (Variables|Default|GetEyeRight))) false)
    (return)
    (else
      (Development|PrintString "Warning: Received partial blob")
      (return))))

(fn UpdateBlendShape
  (params (Array :type Array%20of%20Osc%20Data%20Elem%20Struct%20Structures))
  (bind _output (Utilities|Array|Get(acopy) Array))
  (bind _output_2 (Utilities|Array|Get(acopy) Array 1))
  (bind _returnvalue (Class|OscFunctionLibrary|AsInt _output))
  (bind _returnvalue_2 (Class|OscFunctionLibrary|AsFloat _output_2))
  (if (== (Utilities|Array|Length Array) 2)
    (Utilities|Array|SetArrayElem (Variables|Default|GetMorphValues) _returnvalue _returnvalue_2)
    (Development|PrintString (Utilities|String|Append "Blendshape: " (Utilities|String|ToString(Integer) _returnvalue) "=" (Utilities|String|ToString(Float) _returnvalue_2)) false)
    (return)
    (else
      (Development|PrintString "Warning: Received partial blob")
      (return))))